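; Player controller that drives the BP_CamDrone camera pawn with mouse edge scrolling and wheel zoom.
; On BeginPlay it caches the possessed drone as CurrentCamera, then each Tick sends it scroll input scaled by ScrollSpeed and delta time.
; GetMouseScroll returns zero outside the viewport-edge threshold band, ramps linearly with depth into it, and inverts the Y axis.
; Mouse wheel presses call the drone's zoom in and out functions.
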(event EventBeginPlay
  (bind _asbp_cam_drone (Utilities|Casting|CastToBP_CamDrone (Pawn|GetControlledPawn)))
  (Variables|Default|SetCurrentCamera _asbp_cam_drone))

(event EventTick
  (params (DeltaSeconds :type Float%20%28single-precision%29))
  (bind (_scroll_x _scroll_y) (CallFunction|GetMouseScroll))
  (bind _scrollspeed (Variables|Default|GetScrollSpeed))
  (Default|ScrollScreen (Variables|Default|GetCurrentCamera) (* _scroll_x DeltaSeconds _scrollspeed) (* _scroll_y DeltaSeconds _scrollspeed)))

(event Input|MouseEvents|MouseWheelUp
  (params (Key :type Key%20Structure))
  (:Pressed
    (Default|ZoominScreen (Variables|Default|GetCurrentCamera))))

(event Input|MouseEvents|MouseWheelDown
  (params (Key :type Key%20Structure))
  (:Pressed
    (Default|ZoomOutScreen (Variables|Default|GetCurrentCamera))))

(fn ConstructionScript)

(fn GetMouseScroll
  (bind (_locationx _locationy _returnvalue) (Game|Player|GetMousePosition))
  (bind _returnvalue_2 (Viewport|GetViewportSize))
  (bind _mousescrollthreshold (Variables|Default|GetMouseScrollThreshold))
  (bind (_x _y) (Math|Vector2D|BreakVector2D _returnvalue_2))
  (bind _returnvalue_3 (- 0.5 _mousescrollthreshold))
  (bind _returnvalue_4 (/ _locationx _x))
  (bind _returnvalue_5 (/ _locationy _y))
  (bind _returnvalue_6 (- _returnvalue_4 0.5))
  (bind _returnvalue_7 (- _returnvalue_5 0.5))
  (return (Math|Float|SelectFloat (* (- _returnvalue_6 (* (Math|Float|Sign(Float) _returnvalue_6) _returnvalue_3)) 1e+01) 0.0 (and _returnvalue (>= (Math|Float|Absolute(Float) _returnvalue_6) _returnvalue_3))) (Math|Float|SelectFloat (* (- (* _returnvalue_3 (Math|Float|Sign(Float) _returnvalue_7)) _returnvalue_7) 1e+01) 0.0 (and _returnvalue (>= (Math|Float|Absolute(Float) _returnvalue_7) _returnvalue_3)))))