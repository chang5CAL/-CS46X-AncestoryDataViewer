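; BP_CamDrone is a camera drone actor that frames, pans and zooms the 2D layout built by BP_twoD_NodeSpawner.
; Tick sets a fixed rotation and retries until the last spawner found reports non-zero Screenlevel and Middle, then positions the drone from them once.
; ScrollScreen pans in X and Z within the CamBorder limits.
; Zoom functions step along Y without clamping, and SetActorNewLocation moves it to any given point.
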(event EventBeginPlay)

(event Collision|EventActorBeginOverlap
  (params (OtherActor :type Actor%20Object%20Reference)))

(event EventTick
  (params (DeltaSeconds :type Float%20%28single-precision%29))
  (if (not (Variables|Default|GethasRun))
    (Utilities|FlowControl|Sequence
      (:then_0
        (Transformation|SetActorRotation "0,-90.000000, 0"))
      (:then_1
        (bind _outactors (Actor|GetAllActorsOfClass "/Game/Blueprints/BP_twoD_NodeSpawner.BP_twoD_NodeSpawner_C"))
        (for _array_element _outactors
          _)
        (Math|Float|CompareFloat (Variables|/Script/ADVR.twoD_NodeSpawner|GetScreenlevel _array_element) 0.0
          (:>
            _)
          (:<
            _))
        (Math|Float|CompareFloat (Variables|/Script/ADVR.twoD_NodeSpawner|Getmiddle _array_element) 0.0
          (:>
            _)
          (:<
            _))
        (Variables|Default|SethasRun true)
        (Transformation|SetActorLocation (Math|Vector|MakeVector (Variables|/Script/ADVR.twoD_NodeSpawner|Getmiddle _array_element) (* (Variables|/Script/ADVR.twoD_NodeSpawner|Getmiddle _array_element) 0.4) (* (Variables|/Script/ADVR.twoD_NodeSpawner|GetScreenlevel _array_element) 1.5e+02)) false false)))))

(fn ConstructionScript)

(fn ScrollScreen
  (params (X :type Float%20%28single-precision%29) (Y :type Float%20%28single-precision%29))
  (bind _returnvalue (Transformation|GetActorLocation))
  (bind (_x _y _z) (Math|Vector|BreakVector _returnvalue))
  (Transformation|SetActorLocation (Math|Vector|MakeVector (Math|Float|Clamp(Float) (+ _x X) (Variables|Default|GetCamBorder_Left) (Variables|Default|GetCamBorder_Right)) _y (Math|Float|Clamp(Float) (+ _z Y) (Variables|Default|GetCamBorder_Bottom) (Variables|Default|GetCamBorder_Top))) false false))

(fn SetActorNewLocation
  (params (X :type Float%20%28single-precision%29) (Y :type Float%20%28single-precision%29) (Z :type Float%20%28single-precision%29))
  (Transformation|SetActorLocation (Math|Vector|MakeVector X Y Z) false false))

(fn ZoominScreen
  (bind _returnvalue (Transformation|GetActorLocation))
  (bind (_x _y _z) (Math|Vector|BreakVector _returnvalue))
  (Transformation|SetActorLocation (Math|Vector|MakeVector _x (+ -5e+01 _y) _z) false false))

(fn ZoomOutScreen
  (bind _returnvalue (Transformation|GetActorLocation))
  (bind (_x _y _z) (Math|Vector|BreakVector _returnvalue))
  (Transformation|SetActorLocation (Math|Vector|MakeVector _x (+ 5e+01 _y) _z) false false))