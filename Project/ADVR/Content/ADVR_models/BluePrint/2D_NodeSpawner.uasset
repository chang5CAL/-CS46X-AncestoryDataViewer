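; Actor Blueprint that links the game instance's file name and person selection to a common-ancestor search; no spawning logic appears in its graphs.
; BeginPlay copies FileName from DataGameInstance into FName.
; Tick polls Buttonpressed and, while it is true, calls FindCommonAncestor on Person2 and Person1 with a debug print, without resetting the flag here.
; Two custom events remain as stubs, one empty and one printing the file name.
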(event Custom|CustomEvent
  (params (DeltaSeconds :type Float%20%28single-precision%29)))

(event Custom|CustomEvent_1
  (params (DeltaSeconds :type Float%20%28single-precision%29))
  (bind _asdata_game_instance (Utilities|Casting|CastToDataGameInstance (Game|GetGameInstance)))
  (Development|PrintString (Variables|/Game/Blueprints/DataGameInstance.DataGameInstance_C|GetFileName _asdata_game_instance)))

(event EventBeginPlay
  (bind _asdata_game_instance (Utilities|Casting|CastToDataGameInstance (Game|GetGameInstance)))
  (Variables|Default|SetfName (Variables|/Game/Blueprints/DataGameInstance.DataGameInstance_C|GetFileName _asdata_game_instance)))

(event Collision|EventActorBeginOverlap
  (params (OtherActor :type Actor%20Object%20Reference)))

(event EventTick
  (params (DeltaSeconds :type Float%20%28single-precision%29))
  (bind _asdata_game_instance (Utilities|Casting|CastToDataGameInstance (Game|GetGameInstance)))
  (if (Variables|/Game/Blueprints/DataGameInstance.DataGameInstance_C|Getbuttonpressed _asdata_game_instance)
    (bind _asdata_game_instance_2 (Utilities|Casting|CastToDataGameInstance (Game|GetGameInstance)))
    (bind _asdata_game_instance_3 (Utilities|Casting|CastToDataGameInstance (Game|GetGameInstance)))
    (Class|TwoDNodeSpawner|FindCommonAncestor (Variables|/Game/Blueprints/DataGameInstance.DataGameInstance_C|GetPerson2 _asdata_game_instance_3) (Variables|/Game/Blueprints/DataGameInstance.DataGameInstance_C|GetPerson1 _asdata_game_instance_2))
    (Development|PrintString "Hello")))

(fn ConstructionScript)