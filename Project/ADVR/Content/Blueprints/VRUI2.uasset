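; VR player actor for a lineage viewer that handles motion-controller movement and person selection, and spawns a DataDisplay attached to the camera manager.
; Thumbsticks offset the actor along camera axes, while triggers and grips step two person IDs in DataGameInstance.
; Left face buttons zero-pad IDs for BP_twoD_NodeSpawner, either storing the pair's common ancestor or opening 3D_lineage_map for the first person.
; Right face buttons exit the game.
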(event EventBeginPlay
  (bind _returnvalue (Game|SpawnActorfromClass "/Game/Blueprints/DataDisplay.DataDisplay_C" (Math|Transform|MakeTransform "180.000000,90.000000,-60.000000" "-90.000000,0.000000,-180.000000" "0.300000,0.300000,0.300000") "AlwaysSpawn" 0 0))
  (Transformation|AttachActorToActor _returnvalue (Game|GetPlayerCameraManager 0) "None" "KeepWorld" "KeepWorld" "KeepWorld" true))

(event Collision|EventActorBeginOverlap
  (params (OtherActor :type Actor%20Object%20Reference)))

(event EventTick
  (params (DeltaSeconds :type Float%20%28single-precision%29)))

(event Input|KeyboardEvents|MotionControllerLeftThumbstickX
  (params (AxisValue :type Float%20%28single-precision%29))
  (Transformation|AddActorLocalOffset (* (Math|Vector|ProjectVectorontoPlane (Math|Vector|GetRightVector (Variables|Default|GetCamera)) "0, 0,1.000000") (* AxisValue 4.0)) false false))

(event Input|KeyboardEvents|MotionControllerLeftThumbstickY
  (params (AxisValue :type Float%20%28single-precision%29))
  (Transformation|AddActorLocalOffset (* (Math|Vector|ProjectVectorontoPlane (Math|Vector|GetForwardVector (Variables|Default|GetCamera)) "0, 0,1.000000") (* AxisValue -4.0)) false false))

(event Input|KeyboardEvents|MotionControllerRightThumbstickY
  (params (AxisValue :type Float%20%28single-precision%29))
  (Transformation|AddActorLocalOffset (* (Math|Vector|ProjectVectorontoPlane (Math|Vector|GetUpVector (Variables|Default|GetCamera)) "0, 0, 0") (* AxisValue -4.0)) false false))

(event Input|KeyboardEvents|MotionControllerLeftGrip1
  (params (Key :type Key%20Structure))
  (:Pressed
    (bind _asdata_game_instance (Utilities|Casting|CastToDataGameInstance (Game|GetGameInstance)))
    (Math|Integer|DecrementInt (Variables|/Game/Blueprints/DataGameInstance.DataGameInstance_C|GetVRPerson1 _asdata_game_instance))))

(event Input|KeyboardEvents|MotionControllerLeftTrigger
  (params (Key :type Key%20Structure))
  (:Pressed
    (bind _asdata_game_instance (Utilities|Casting|CastToDataGameInstance (Game|GetGameInstance)))
    (Math|Integer|IncrementInt (Variables|/Game/Blueprints/DataGameInstance.DataGameInstance_C|GetVRPerson1 _asdata_game_instance))))

(event Input|KeyboardEvents|MotionControllerRightFaceButton2
  (params (Key :type Key%20Structure))
  (:Pressed
    (Development|ExecuteConsoleCommand "EXIT")))

(event Input|KeyboardEvents|MotionControllerRightGrip1
  (params (Key :type Key%20Structure))
  (:Pressed
    (bind _asdata_game_instance (Utilities|Casting|CastToDataGameInstance (Game|GetGameInstance)))
    (Math|Integer|DecrementInt (Variables|/Game/Blueprints/DataGameInstance.DataGameInstance_C|GetVRPerson2 _asdata_game_instance))))

(event Input|KeyboardEvents|MotionControllerRightFaceButton1
  (params (Key :type Key%20Structure))
  (:Pressed
    (Development|ExecuteConsoleCommand "EXIT")))

(event Input|KeyboardEvents|MotionControllerRightTrigger
  (params (Key :type Key%20Structure))
  (:Pressed
    (bind _asdata_game_instance (Utilities|Casting|CastToDataGameInstance (Game|GetGameInstance)))
    (Math|Integer|IncrementInt (Variables|/Game/Blueprints/DataGameInstance.DataGameInstance_C|GetVRPerson2 _asdata_game_instance))))

(event Input|KeyboardEvents|MotionControllerLeftFaceButton1
  (params (Key :type Key%20Structure))
  (:Pressed
    (bind _outactors (Actor|GetAllActorsOfClass "/Game/Blueprints/BP_twoD_NodeSpawner.BP_twoD_NodeSpawner_C"))
    (for _array_element _outactors
      _)
    (bind _asdata_game_instance (Utilities|Casting|CastToDataGameInstance (Game|GetGameInstance)))
    (bind _id (CallFunction|ConvertIntIDtoStringID (Variables|/Game/Blueprints/DataGameInstance.DataGameInstance_C|GetVRPerson1 _asdata_game_instance)))
    (bind _id_2 (CallFunction|ConvertIntIDtoStringID (Variables|/Game/Blueprints/DataGameInstance.DataGameInstance_C|GetVRPerson2 _asdata_game_instance)))
    (bind _returnvalue (Class|TwoDNodeSpawner|FindCommonAncestor _array_element _id _id_2))
    (bind _asdata_game_instance_2 (Utilities|Casting|CastToDataGameInstance (Game|GetGameInstance)))
    (Variables|/Game/Blueprints/DataGameInstance.DataGameInstance_C|SetAncestryData _asdata_game_instance_2 _returnvalue)))

(event Input|KeyboardEvents|MotionControllerLeftFaceButton2
  (params (Key :type Key%20Structure))
  (:Pressed
    (bind _outactors (Actor|GetAllActorsOfClass "/Game/Blueprints/BP_twoD_NodeSpawner.BP_twoD_NodeSpawner_C"))
    (for _array_element _outactors
      _)
    (bind _asdata_game_instance (Utilities|Casting|CastToDataGameInstance (Game|GetGameInstance)))
    (bind _id (CallFunction|ConvertIntIDtoStringID (Variables|/Game/Blueprints/DataGameInstance.DataGameInstance_C|GetVRPerson1 _asdata_game_instance)))
    (Class|TwoDNodeSpawner|CheckValidPerson _array_element _id)
    (if true
      (bind _asdata_game_instance_2 (Utilities|Casting|CastToDataGameInstance (Game|GetGameInstance)))
      (Variables|/Game/Blueprints/DataGameInstance.DataGameInstance_C|SetPerson1 _asdata_game_instance_2 _id)
      (Game|OpenLevel(byName) "3D_lineage_map"))))

(fn ConstructionScript)

(fn ConvertIntIDtoStringID
  (params (IntID :type Integer))
  (Math|Integer|CompareInt IntID 10
    (:>
      _)
    (:==
      _)
    (:<
      (return (Utilities|String|Append "0" (Utilities|String|ToString(Integer) IntID)))))
  (return (Utilities|String|ToString(Integer) IntID)))