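; DataDisplay is an actor Blueprint that shows session data from the game instance on three text components.
; Every tick it casts the game instance to DataGameInstance and writes the VRPerson1 and VRPerson2 integers and the AncestryData value into IDPerson1, IDPerson2 and AncestryText.
; The text is refreshed by per-frame polling, and BeginPlay, overlap and construction logic are empty.
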(event EventBeginPlay)

(event Collision|EventActorBeginOverlap
  (params (OtherActor :type Actor%20Object%20Reference)))

(event EventTick
  (params (DeltaSeconds :type Float%20%28single-precision%29))
  (bind _asdata_game_instance (Utilities|Casting|CastToDataGameInstance (Game|GetGameInstance)))
  (Rendering|Components|TextRender|SetText (Variables|Default|GetIDPerson1) (Utilities|Text|ToText(Integer) (Variables|/Game/Blueprints/DataGameInstance.DataGameInstance_C|GetVRPerson1 _asdata_game_instance)))
  (Rendering|Components|TextRender|SetText (Variables|Default|GetIDPerson2) (Utilities|Text|ToText(Integer) (Variables|/Game/Blueprints/DataGameInstance.DataGameInstance_C|GetVRPerson2 _asdata_game_instance)))
  (Rendering|Components|TextRender|SetText (Variables|Default|GetAncestryText) (Utilities|Text|ToText(String) (Variables|/Game/Blueprints/DataGameInstance.DataGameInstance_C|GetAncestryData _asdata_game_instance))))

(fn ConstructionScript)