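; VR UI actor for a lineage screen that shows an instructions actor and handles motion-controller navigation.
; On BeginPlay it spawns LineageInstructions and attaches it to the player camera manager.
; The left thumbstick moves the actor horizontally relative to the camera, the right along camera up, while face buttons open 3D_map (left) or exit the game (right).
; A helper function zero-pads integer IDs below ten into strings.
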(event EventBeginPlay
  (bind _returnvalue (Game|SpawnActorfromClass "/Game/Blueprints/LineageInstructions.LineageInstructions_C" (Math|Transform|MakeTransform "180.000000,90.000000,-60.000000" "-90.000000,0.000000,-180.000000" "0.300000,0.300000,0.300000") "AlwaysSpawn" 0 0))
  (Transformation|AttachActorToActor _returnvalue (Game|GetPlayerCameraManager 0) "None" "KeepWorld" "KeepWorld" "KeepWorld" true))

(event Collision|EventActorBeginOverlap
  (params (OtherActor :type Actor%20Object%20Reference)))

(event EventTick
  (params (DeltaSeconds :type Float%20%28single-precision%29)))

(event Input|KeyboardEvents|MotionControllerLeftThumbstickX
  (params (AxisValue :type Float%20%28single-precision%29))
  (Transformation|AddActorLocalOffset (* (Math|Vector|ProjectVectorontoPlane (Math|Vector|GetRightVector (Variables|Default|GetCamera)) "0, 0,1.000000") (* AxisValue 4.0)) false false))

(event Input|KeyboardEvents|MotionControllerLeftThumbstickY
  (params (AxisValue :type Float%20%28single-precision%29))
  (Transformation|AddActorLocalOffset (* (Math|Vector|ProjectVectorontoPlane (Math|Vector|GetForwardVector (Variables|Default|GetCamera)) "0, 0,1.000000") (* AxisValue -4.0)) false false))

(event Input|KeyboardEvents|MotionControllerRightThumbstickY
  (params (AxisValue :type Float%20%28single-precision%29))
  (Transformation|AddActorLocalOffset (* (Math|Vector|ProjectVectorontoPlane (Math|Vector|GetUpVector (Variables|Default|GetCamera)) "0, 0, 0") (* AxisValue -4.0)) false false))

(event Input|KeyboardEvents|MotionControllerRightFaceButton2
  (params (Key :type Key%20Structure))
  (:Pressed
    (Development|ExecuteConsoleCommand "EXIT")))

(event Input|KeyboardEvents|MotionControllerRightFaceButton1
  (params (Key :type Key%20Structure))
  (:Pressed
    (Development|ExecuteConsoleCommand "EXIT")))

(event Input|KeyboardEvents|MotionControllerLeftFaceButton1
  (params (Key :type Key%20Structure))
  (:Pressed
    (Game|OpenLevel(byName) "3D_map")))

(event Input|KeyboardEvents|MotionControllerLeftFaceButton2
  (params (Key :type Key%20Structure))
  (:Pressed
    (Game|OpenLevel(byName) "3D_map")))

(fn ConstructionScript)

(fn ConvertIntIDtoStringID
  (params (IntID :type Integer))
  (Math|Integer|CompareInt IntID 10
    (:>
      _)
    (:==
      _)
    (:<
      (return (Utilities|String|Append "0" (Utilities|String|ToString(Integer) IntID)))))
  (return (Utilities|String|ToString(Integer) IntID)))